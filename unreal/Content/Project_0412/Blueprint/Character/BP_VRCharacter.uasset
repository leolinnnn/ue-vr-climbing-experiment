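; VR player character Blueprint that handles thumbstick locomotion and turning through Enhanced Input.
; The left stick adds movement input, with both X and Y axes applied along the VR forward vector.
; The right stick snap-turns through the VR movement component past a deadzone, gated by a Turn flag that is set on release but never cleared here.
; Right-controller grip and drop calls are present but unwired.
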(event Input|EnhancedActionEvents|EnhancedInputActionIA_LeftThumbAxis
  (params (ActionValue :type Vector%202D%20Structure) (ElapsedSeconds :type Float%20%28double-precision%29) (TriggeredSeconds :type Float%20%28double-precision%29) (InputAction :type Input%20Action%20Object%20Reference :default "/Game/Project_0412/Input/IA_LeftThumbAxis.IA_LeftThumbAxis"))
  ;[1 1 1] movement
  (Pawn|Input|AddMovementInput (Class|VRBaseCharacter|GetVRForwardVector) (.y ActionValue) false)
  (Pawn|Input|AddMovementInput (Class|VRBaseCharacter|GetVRForwardVector) (.x ActionValue) false))

(event Input|EnhancedActionEvents|EnhancedInputActionIA_RightThumbAxis
  (params (ActionValue :type Vector%202D%20Structure) (ElapsedSeconds :type Float%20%28double-precision%29) (TriggeredSeconds :type Float%20%28double-precision%29) (InputAction :type Input%20Action%20Object%20Reference :default "/Game/Project_0412/Input/IA_RightThumbAxis.IA_RightThumbAxis"))
  (bind _snap_turn_delta_yaw (Variables|Default|GetSnap%20Turn%20Delta%20Yaw))
  ;[1 1 1] turn
  (:Triggered
    (if (and (> (Math|Float|Absolute(Float) (.x ActionValue)) 0.5) (Variables|Default|Getturn))
      (Class|VRBaseCharacterMovementComponent|PerformMoveActionSnapTurn (Variables|Default|GetVRMovementReference) (Math|Float|SelectFloat _snap_turn_delta_yaw (* _snap_turn_delta_yaw -1.0) (> (.x ActionValue) 0.0)) "VRMOVEACTION_Velocity_None" false false true)))
  (:Completed
    (Variables|Default|Setturn true)))

(event EventBeginPlay)

(event Collision|EventActorBeginOverlap
  (params (OtherActor :type Actor%20Object%20Reference)))

(event EventTick
  (params (DeltaSeconds :type Float%20%28single-precision%29)))

(fn ConstructionScript)